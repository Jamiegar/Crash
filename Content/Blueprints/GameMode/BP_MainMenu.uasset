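; Main menu Blueprint that sets up local players, the camera view and the menu UI on BeginPlay.
; It first creates a second local player with Game and UI input.
; If the level has a CineCameraActor, it makes that the first player's view target and adds WBP_MenuMaster to the viewport.
; The menu belongs to the first player, who gets Game and UI input with a hidden cursor.
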(event `self.ReceiveBeginPlay`
  (`self.SpawnAdditionalController`)
  (bind _returnvalue (`GameplayStatics.GetActorOfClass` "/Script/CinematicCamera.CineCameraActor"))
  (`/Engine/EditorBlueprintResources/StandardMacros.IsValid` _returnvalue
    (:`Is Valid`
      (`PlayerController.SetViewTargetWithBlend` (`GameplayStatics.GetPlayerController` 0) _returnvalue 0.0 "VTBlend_Linear" 0.0 false)
      (`self.CreateMainMenu`))))

(event `SpawnAdditionalController`
  (bind _returnvalue (`GameplayStatics.CreatePlayer` 1))
  (`WidgetBlueprintLibrary.SetInputMode_GameAndUIEx` _returnvalue null))

(fn `CreateMainMenu`
  (bind _returnvalue (`GameplayStatics.GetPlayerController` 0))
  (bind _returnvalue_2 (`|CreateWidget` "/Game/Blueprints/UserInterface/Menu/WBP_MenuMaster.WBP_MenuMaster_C" (`GameplayStatics.GetPlayerController` 0)))
  (`UserWidget.AddToViewport` _returnvalue_2 0)
  (set `PlayerController.bShowMouseCursor` false _returnvalue)
  (`WidgetBlueprintLibrary.SetInputMode_GameAndUIEx` _returnvalue null))

(fn `UserConstructionScript`)