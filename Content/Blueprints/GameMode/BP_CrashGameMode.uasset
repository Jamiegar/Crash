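; BP_CrashGameMode is the game mode that runs the match flow for a character knockout game.
; Setup locks input on all active characters and runs an optional countdown widget, whose finish event restores input, creates the main UI and fades in music.
; A knockout replaces all widgets with a winner-aware end screen and fades music out.
; Two pause events share one function that toggles game pause and plays the pause menu's intro or outro.
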(event `self.GameSetUp`
  (`GameplayStatics.PlaySound2D` "/Game/Assets/Ultimate_SFX/Impacts_Sweeps/Cues/Impact_01_Cue.Impact_01_Cue" 1.0 1.0 0.0 null null)
  (for _array_element (`self.ActiveCharacters`)
    (`self.DisableInput` _array_element (cast `PlayerController` (`Pawn.GetController` _array_element) :!pure true)))
  (`self.StartGameCountDown`))

(event `StartGameCountDown`
  (if (`self.EnableCountdown`)
    (bind _returnvalue (`|CreateWidget` "/Game/Blueprints/UserInterface/Game/WBP_CountDown.WBP_CountDown_C"))
    (`UserWidget.AddToViewport` _returnvalue 0)
    (add `/Game/Blueprints/UserInterface/Game/WBP_CountDown.OnCountdownFinished` _returnvalue (delegate `OnCountdownFinished`))
    (message `/Game/Blueprints/UserInterface/Menu/BPI_UserInterface.BeginIntro` _returnvalue)
    (else
      (for _array_element (`self.ActiveCharacters`) :!label _label
        (`self.EnableInput` _array_element (cast `PlayerController` (`Pawn.GetController` _array_element) :!pure true)))
      (`self.CreateMainUI`)
      (bind _returnvalue_2 (`GameplayStatics.SpawnSound2D` "/Game/Blueprints/MetaSounds/Music/MS_GameMusic.MS_GameMusic" 1.0 1.0 0.0 null))
      (bind _output_get (set `self.GameMusic` _returnvalue_2))
      (`AudioComponent.FadeIn` _output_get 0.2 1.0 0.0 "Linear"))))

(event `OnCountdownFinished`
  (goto _label))

(event `self.OnCharacterKnockedOut`
  (params (WinningCharacter :type "PlayerController Object Reference"))
  (`WidgetLayoutLibrary.RemoveAllWidgets`)
  (bind _returnvalue (`|CreateWidget` "/Game/Blueprints/UserInterface/GameFinishedMenu/UI_MasterGameEnd.UI_MasterGameEnd_C" null WinningCharacter))
  (`UserWidget.AddToViewport` _returnvalue 0)
  (`AudioComponent.FadeOut` (`self.GameMusic`) 1.5 0.0 "Linear"))

(event `self.SetGamePause`
  (params (IsPaused :type Boolean))
  (`self.SetGameupForPause` IsPaused))

(event `SetCrashGamePaused`
  (params (IsPaused :type Boolean))
  (`self.SetGameupForPause` IsPaused))

(fn `CreateMainUI`
  (bind _returnvalue (`|CreateWidget` "/Game/Blueprints/UserInterface/Game/WBP_GameMaster.WBP_GameMaster_C" null (`self.ActiveCharacters`)))
  (`UserWidget.AddToViewport` _returnvalue 0))

(fn `SetGameupForPause`
  (params (bPaused :type Boolean))
  (`GameplayStatics.SetGamePaused` bPaused)
  (if bPaused
    (bind _returnvalue (`|CreateWidget` "/Game/Blueprints/UserInterface/PauseMenu/WBP_MainPauseMenu.WBP_MainPauseMenu_C" (`GameplayStatics.GetPlayerController` 0)))
    (bind _output_get (set `self.PauseMenu` _returnvalue))
    (message `/Game/Blueprints/UserInterface/Menu/BPI_UserInterface.BeginIntro` _output_get)
    (else
      (message `/Game/Blueprints/UserInterface/Menu/BPI_UserInterface.BeginOutro` (`self.PauseMenu`)))))

(fn `UserConstructionScript`)